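; Test inspect actor: Interact freezes the player's movement and look, shows the cursor and lets the mouse rotate the Cube.
; A Timeline lerps the Cube's rotation toward the character's Sphere, while the location lerp's alpha stays at 0, holding its start position.
; Tick and mouse axis events share the rotation logic, gated by CanInspect.
; The A key resets the DoOnce and restores controls without returning the Cube's transform.
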(event `self.ReceiveBeginPlay`
  (bind _cube (`self.Cube`))
  ; systeme d'inspect
  ;; récup les positions
  (bind _output_get (set `self.Position d'origine` (`SceneComponent.K2_GetComponentLocation` _cube)))
  (bind _output_get_2 (set `self.rotation d'origine` (`SceneComponent.K2_GetComponentRotation` _cube)))
  (`self.EnableInput` (`GameplayStatics.GetPlayerController` 0)))

(event `/Game/ProjetDeFouMalade/BPI_Interact.Interact`
  ; systeme d'inspect
  (`/Engine/EditorBlueprintResources/StandardMacros.DoOnce` false :!label _label
    (:`Completed`
      (set `PlayerController.bShowMouseCursor` true (`GameplayStatics.GetPlayerController` 0))
      (set `self.can Inspect ?` true)
      (bind _asbp_first_person_character (cast `/Game/FirstPerson/Blueprints/BP_FirstPersonCharacter` (`GameplayStatics.GetPlayerCharacter` 0)))
      (`CharacterMovementComponent.DisableMovement` (`Character.CharacterMovement` (`GameplayStatics.GetPlayerCharacter` 0)))
      (`Controller.SetIgnoreLookInput` (`GameplayStatics.GetPlayerController` 0) true)
      (bind (_direction _newtrack_0) (`Timeline|Timeline`)
        (:`Update`
          (bind (_returnvalue_location _returnvalue_rotation) (`KismetMathLibrary.BreakTransform` (`SceneComponent.K2_GetComponentToWorld` (`/Game/FirstPerson/Blueprints/BP_FirstPersonCharacter.Sphere` _asbp_first_person_character))))
          (`SceneComponent.K2_SetWorldTransform` (`self.Cube`) (`KismetMathLibrary.MakeTransform` (`KismetMathLibrary.VLerp` (stale `self.ReceiveBeginPlay` _output_get) _returnvalue_location) (`KismetMathLibrary.RLerp` (stale `self.ReceiveBeginPlay` _output_get_2) _returnvalue_rotation _newtrack_0)) false false))))))

(event `Key|A`
  (params (Key :type "Key Structure"))
  (bind _returnvalue (`GameplayStatics.GetPlayerController` 0))
  ; systeme d'inspect
  ;; enlever l'inspect
  (:`Pressed`
    (`|ExecutionSequence`
      (:`then_0`
        (goto _label :!via `Reset`))
      (:`then_1`
        (set `self.can Inspect ?` false)
        (`CharacterMovementComponent.SetMovementMode` (`Character.CharacterMovement` (`GameplayStatics.GetPlayerCharacter` 0)) "MOVE_Walking" 0)
        (set `PlayerController.bShowMouseCursor` false _returnvalue)
        (`Controller.ResetIgnoreLookInput` _returnvalue)
        (`WidgetBlueprintLibrary.SetInputMode_GameOnly` _returnvalue)))))

(event `self.ReceiveTick`
  (params (DeltaSeconds :type "Float (single-precision)"))
  ; systeme d'inspect
  ;; rOTATION
  (if (`self.can Inspect ?`) :!label _label_2
    (`SceneComponent.K2_AddLocalRotation` (`self.Cube`) (`KismetMathLibrary.MakeRotator` (* (stale `InputAxisKey|MouseX` AxisValue) 1.0) (* (stale `InputAxisKey|MouseY` AxisValue) 1.0)) false false)))

(event `InputAxisKey|MouseX`
  (params (AxisValue :type "Float (single-precision)"))
  ; systeme d'inspect
  ;; rOTATION
  (goto _label_2))

(event `InputAxisKey|MouseY`
  (params (AxisValue :type "Float (single-precision)"))
  ; systeme d'inspect
  ;; rOTATION
  (goto _label_2))

(fn `UserConstructionScript`)