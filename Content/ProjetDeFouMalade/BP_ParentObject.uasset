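; Base actor for interactable objects that the first-person player can inspect up close.
; Inspection blocks player movement, makes the capsule ignore WorldDynamic, and lerps the object from its starting transform to the player's inspection sphere and camera rotation via a timeline.
; Stopping reverses that timeline.
; An icon widget can be shown or hidden, with range events using DoOnce gates to control its animation.
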(event `self.ReceiveBeginPlay`
  (set `self.InitialPosition` (`SceneComponent.K2_GetComponentToWorld` (`self.DefaultSceneRoot`)))
  (if (`self.ActorHasTag` "IsBook")
    (bind _asbp_first_person_character (cast `/Game/FirstPerson/Blueprints/BP_FirstPersonCharacter` (`GameplayStatics.GetPlayerCharacter` 0)))
    (bind _output_get (set `self.FPC_Ref` _asbp_first_person_character))))

(event `/Game/ProjetDeFouMalade/BPI_Interact.ObjectInspection`
  (bind (_initialposition_location _initialposition_rotation) (`KismetMathLibrary.BreakTransform` (`self.InitialPosition`)))
  (bind _asbp_first_person_character (cast `/Game/FirstPerson/Blueprints/BP_FirstPersonCharacter` (`GameplayStatics.GetPlayerCharacter` 0)))
  (`PrimitiveComponent.SetCollisionResponseToChannel` (`Character.CapsuleComponent` _asbp_first_person_character) "ECC_WorldDynamic" "ECR_Ignore")
  (set `/Game/FirstPerson/Blueprints/BP_FirstPersonCharacter.bIsInspecting` true _asbp_first_person_character)
  (set `/Game/FirstPerson/Blueprints/BP_FirstPersonCharacter.bCanMove` false _asbp_first_person_character)
  (bind (_direction _move) (`Timeline|MoveObject` :!label _label)
    (:`Update`
      (`self.K2_SetActorLocationAndRotation` (`KismetMathLibrary.VLerp` _initialposition_location (`SceneComponent.K2_GetComponentLocation` (`/Game/FirstPerson/Blueprints/BP_FirstPersonCharacter.Sphere1` _asbp_first_person_character)) _move) (`KismetMathLibrary.RLerp` _initialposition_rotation (`SceneComponent.K2_GetComponentRotation` (`/Game/FirstPerson/Blueprints/BP_FirstPersonCharacter.FirstPersonCamera` _asbp_first_person_character)) _move)))
    (:`Finished`
      (`/Game/FirstPerson/Blueprints/BP_FirstPersonCharacter.TimelineFinished` _asbp_first_person_character))))

(event `/Game/ProjetDeFouMalade/BPI_Interact.StopObjectInspection`
  (goto _label :!via `Reverse`))

(event `/Game/ProjetDeFouMalade/BPI_ITEM.ActiveWidget`
  ;[0.03055 0.15 0.04108 0.5] Affiche le widget sur les objets [Maelik]
  (`SceneComponent.SetVisibility` (`self.Widget`) true false))

(event `/Game/ProjetDeFouMalade/BPI_ITEM.HideWidget`
  ;[0.03055 0.15 0.04108 0.5] Affiche le widget sur les objets [Maelik]
  (`SceneComponent.SetVisibility` (`self.Widget`) false false))

(event `/Game/ProjetDeFouMalade/BPI_ITEM.InRangeInteract`
  ;[0.03055 0.15 0.04108 0.5] Fais apparaitre et disparaitre le widget quand le joueur n'est plus dans le champ de collision de l'objet [Maelik]
  (`/Engine/EditorBlueprintResources/StandardMacros.DoOnce` false :!label _label_2
    (:`Completed`
      (bind _aswb_icone (cast `/Game/Widgets/WB_Icone` (`WidgetComponent.GetUserWidgetObject` (`self.Widget`))))
      (`/Game/Widgets/WB_Icone.LauchAnim` _aswb_icone true)
      (goto _label_3 :!via `Reset`))))

(event `/Game/ProjetDeFouMalade/BPI_ITEM.OutRangeInteract`
  ;[0.03055 0.15 0.04108 0.5] Fais apparaitre et disparaitre le widget quand le joueur n'est plus dans le champ de collision de l'objet [Maelik]
  (`/Engine/EditorBlueprintResources/StandardMacros.DoOnce` false :!label _label_3
    (:`Completed`
      (bind _aswb_icone (cast `/Game/Widgets/WB_Icone` (`WidgetComponent.GetUserWidgetObject` (`self.Widget`))))
      (`/Game/Widgets/WB_Icone.LauchAnim` _aswb_icone true)
      (goto _label_2 :!via `Reset`))))

(fn `UserConstructionScript`)